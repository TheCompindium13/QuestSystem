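; Base collectible actor that reports to the current quest when BP_ThirdPersonCharacter hits it.
; On each such hit it updates every objective of the game mode's current quest by 1, as the class check in the loop does not filter any out.
; It then swaps its mesh material and stays in the world, with no guard against repeat hits.
; An end-overlap handler sets another material, but its binding never runs.
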(event `self.ReceiveBeginPlay`
  (add `self.OnActorHit` (delegate `OnActorHit_Event`)))

(event `OnActorHit_Event` :!signature `self.OnActorHit`
  (params (SelfActor :type "Actor Object Reference") (OtherActor :type "Actor Object Reference") (NormalImpulse :type "Vector Structure") (Hit :type "HitResult Structure (by ref)"))
  (cast `/Game/ThirdPerson/Blueprints/BP_ThirdPersonCharacter` OtherActor)
  (`self.NotifyCollected`)
  (`PrimitiveComponent.SetMaterial` (`self.StaticMesh`) 0 "/Engine/VREditor/LaserPointer/LaserPointerMaterialInst.LaserPointerMaterialInst"))

(event `self.NotifyCollected`
  (bind _asb_quest_game_blueprint (cast `/Game/QuestBlueprints/B_QuestGameBlueprint` (`GameplayStatics.GetGameMode`)))
  (bind _current_quest_reference (`/Game/QuestBlueprints/B_QuestGameBlueprint.Current Quest Reference` _asb_quest_game_blueprint))
  (for _array_element (`BaseQuest.objectives` _current_quest_reference)
    (if (`KismetMathLibrary.ClassIsChildOf` (`GameplayStatics.GetObjectClass` self) (`GameplayStatics.GetObjectClass` null))
      _
      (else
        _))
    (`BaseQuest.UpdateObjective` _current_quest_reference (`.ObjectiveID` (break `Objective` _array_element)) 1)))

(event `OnActorEndOverlap_Event` :!signature `self.OnActorEndOverlap`
  (params (OverlappedActor :type "Actor Object Reference") (OtherActor :type "Actor Object Reference"))
  (cast `/Game/ThirdPerson/Blueprints/BP_ThirdPersonCharacter` OtherActor)
  (`PrimitiveComponent.SetMaterial` (`self.StaticMesh`) 0 "/Engine/MaterialTemplates/VertexAnimation/AdvancedFlag.AdvancedFlag"))

(fn `UserConstructionScript`)