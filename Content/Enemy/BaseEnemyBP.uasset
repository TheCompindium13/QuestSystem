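; Base enemy Blueprint that credits the current quest when the enemy dies.
; On NotifyDeath it gets the current quest from the B_QuestGameBlueprint game mode and loops through its objectives.
; Each objective whose EnemyToSlay exactly matches this enemy's class is advanced by one through UpdateObjective on the quest.
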(event `self.NotifyDeath`
  (bind _asb_quest_game_blueprint (cast `/Game/QuestBlueprints/B_QuestGameBlueprint` (`GameplayStatics.GetGameMode`)))
  (bind _current_quest_reference (`/Game/QuestBlueprints/B_QuestGameBlueprint.Current Quest Reference` _asb_quest_game_blueprint))
  (for _array_element (`BaseQuest.objectives` _current_quest_reference)
    (bind (_cleartype _enemytoslay _itemtocollect _description _objectiveid) (break `Objective` _array_element))
    (if (== _enemytoslay (`GameplayStatics.GetObjectClass` self))
      (`BaseQuest.UpdateObjective` _current_quest_reference _objectiveid 1))))

(fn `UserConstructionScript`)